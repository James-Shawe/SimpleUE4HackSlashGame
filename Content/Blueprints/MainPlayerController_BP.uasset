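; Player controller Blueprint that animates the pause menu when it is shown and dismissed.
; Both pause events call their parent implementations, then cast PauseMenu to PauseMenu_BP to play its PauseMenuAnimation, forward on display and in reverse on removal.
; After removal, a short delay lets the reverse animation run before the widget is set to Hidden.
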(event EventBeginPlay)

(event EventTick
  (params (DeltaSeconds :type Float%20%28single-precision%29)))

(event EventDisplayPauseMenu
  (|CallParentFunction)
  (bind _aspause_menu_bp (Utilities|Casting|CastToPauseMenu_BP (Variables|Default|GetPauseMenu)))
  (UserInterface|Animation|PlayAnimation _aspause_menu_bp (Variables|/Game/HUD/PauseMenu_BP.PauseMenu_BP_C|GetPauseMenuAnimation _aspause_menu_bp) 0.0 1 "Forward" 1.0 false))

(event EventRemovePauseMenu
  (|CallParentFunction)
  (bind _aspause_menu_bp (Utilities|Casting|CastToPauseMenu_BP (Variables|Default|GetPauseMenu)))
  (UserInterface|Animation|PlayAnimation _aspause_menu_bp (Variables|/Game/HUD/PauseMenu_BP.PauseMenu_BP_C|GetPauseMenuAnimation _aspause_menu_bp) 0.0 1 "Reverse" 1.0 false)
  (Utilities|FlowControl|Delay 0.25)
  (Widget|SetVisibility (Variables|Default|GetPauseMenu) "Hidden"))

(fn ConstructionScript)